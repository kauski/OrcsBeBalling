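; BP_PlaySound is an actor that plays countdown warning and end buzzer sounds through two custom events.
; PlayTimerRunningOut spawns the 2D warning cue and stores its audio component, skipping the spawn while that reference is still valid.
; PlayEndSoundBuzzer stops the stored component if valid, then plays the buzzer horn at the actor's location.
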(event Custom|PlayEndSoundBuzzer
  (Utilities|IsValid (Variables|Default|GetAudioComponentT)
    (:Is%20Valid
      (Audio|Components|Audio|Stop (Variables|Default|GetAudioComponentT)))
    (:Is%20Not%20Valid
      _))
  (Audio|PlaySoundatLocation "/Game/Sounds/SFX_end_buzzer_horn_Cue.SFX_end_buzzer_horn_Cue" (Transformation|GetActorLocation) "0, 0, 0" 1.0 1.0 0.0 0 0 0 0))

(event Custom|PlayTimerRunningOut
  (Utilities|IsValid (Variables|Default|GetAudioComponentT)
    (:Is%20Not%20Valid
      (bind _returnvalue (Audio|SpawnSound2D "/Game/Sounds/SFX_timer_running_out_Cue.SFX_timer_running_out_Cue" 1.0 1.0 0.0 0))
      (Variables|Default|SetAudioComponentT _returnvalue))))

(fn ConstructionScript)