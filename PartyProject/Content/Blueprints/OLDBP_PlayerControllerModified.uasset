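; Player controller for a multiplayer lobby-to-game flow, handling input modes and kicks.
; BeginPlay sets UI-only input; StartGameInputMode switches to game-only and hides every top-level lobby menu widget.
; OC_KickPlayer opens the initial map, then destroys the session.
; UpdatePlayerControllers only reassigns the AllPlayerControllers array to itself, and its OnRep handler is empty.
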(event Custom|StartGameInputMode
  (Input|SetInputModeGameOnly (Game|GetPlayerController 0) false)
  (bind _foundwidgets (Widget|GetAllWidgetsOfClass "/Game/Blueprints/OLDW_LobbyMenu.OLDW_LobbyMenu_C" true))
  (bind _output_get (Variables|Default|SetFound%20Widgets _foundwidgets))
  (for _array_element _output_get
    (bind _asw_lobby_menu (Utilities|Casting|CastToOLDW_LobbyMenu _array_element)
      (:then
        (Default|HIdeLobbyMenu _asw_lobby_menu))
      (:CastFailed
        (Development|PrintString "Hide Lobby Menu CAST FAILED")))))

(event Custom|UpdatePlayerControllers
  (Variables|Default|SetAll%20Player%20Controllers (Variables|Default|GetAll%20Player%20Controllers)))

(event Custom|PreGameInputMode
  (Input|SetInputModeUIOnly (Game|GetPlayerController 0) 0 "DoNotLock" false))

(event Custom|OC_KickPlayer
  ;[1 1 1] Kicks player and loads into initialmap
  (Game|OpenLevel(byName) "L_InitialMap")
  (|DestroySession (Game|GetPlayerController 0)))

(event EventBeginPlay
  (CallFunction|PreGameInputMode))

(fn ConstructionScript)

(fn OnRepAllPlayerControllers)