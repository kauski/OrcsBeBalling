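; Multiplayer party game mode that tracks player controllers, spawns their characters and keeps score.
; Login, seamless swap and logout maintain the controller array, with login renaming players by join order as "p" plus a number.
; SpawnPlayer replaces any existing pawn with a third-person character at the next cached PlayerStart and possesses it.
; GMUpdateScore calls SetScores, which increments the named scorer's counter, one of four, on every controller's own copy.
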(event EventBeginPlay
  (bind _outactors (Actor|GetAllActorsOfClass "/Script/Engine.PlayerStart"))
  (Variables|Default|SetOut%20Actors _outactors)
  (Variables|Default|SetPlayerstart_num 0))

(event EventTick
  (params (DeltaSeconds :type Float%20%28single-precision%29)))

(event EventPostLogin
  (params (NewPlayer :type Player%20Controller%20Object%20Reference))
  (bind _all_partygameplayercontrollers (Variables|Default|GetAll_PartyGamePlayerControllers))
  ;[1 1 1] Connect event
  (Utilities|Array|Add _all_partygameplayercontrollers NewPlayer)
  (bind _foundwidgets (Widget|GetAllWidgetsOfClass "/Game/Blueprints/GameMode/Partygame_UI_Widget.Partygame_UI_Widget_C" true))
  (Variables|Default|SetParygame%20widgets _foundwidgets)
  (for (_array_element _array_index) _all_partygameplayercontrollers
    (bind _aspartygame_multiplayer_playercontroller_bp (Utilities|Casting|CastToPartygame_multiplayer_playercontroller_BP _array_element)
      (:then
        (bind _output_get (Variables|/Game/Blueprints/GameMode/Partygame_multiplayer_playercontroller_BP.Partygame_multiplayer_playercontroller_BP_C|SetIngamename _aspartygame_multiplayer_playercontroller_bp (Utilities|String|Append "p" (Utilities|String|ToString(Integer) (+ _array_index 1)))))
        (Class|AdvancedSessionsLibrary|SetPlayerName _aspartygame_multiplayer_playercontroller_bp _output_get))
      (:CastFailed
        (Development|PrintString "Cast failed in multiplayer gamemode BP" true true "(R=1.000000,G=0.000000,B=0.676688,A=1.000000)" 266.0)))))

(event EventOnSwapPlayerControllers
  (params (OldPC :type Player%20Controller%20Object%20Reference) (NewPC :type Player%20Controller%20Object%20Reference))
  ;[1 1 1] Connect event
  (Utilities|Array|Add (Variables|Default|GetAll_PartyGamePlayerControllers) NewPC))

(event EventOnLogout
  (params (ExitingController :type Controller%20Object%20Reference))
  ;[1 1 1] Disconnect event
  (bind _aspartygame_multiplayer_playercontroller_bp (Utilities|Casting|CastToPartygame_multiplayer_playercontroller_BP ExitingController)
    (:then
      (Utilities|Array|RemoveItem (Variables|Default|GetAll_PartyGamePlayerControllers) _aspartygame_multiplayer_playercontroller_bp))
    (:CastFailed
      (Development|PrintString "Cast failed at Partgame_Multiplayer_gamemode_BP"))))

(fn ConstructionScript)

(fn FindPlayerStartTransform
  (if (>= (Variables|Default|GetPlayerstart_num) 3)
    (Variables|Default|SetPlayerstart_num (Variables|Default|GetPlayerstart_num)))
  (return (Transformation|GetActorTransform (Utilities|Array|Get(acopy) (Variables|Default|GetOut%20Actors) (Variables|Default|GetPlayerstart_num)))))

(fn SpawnPlayer
  (params (PlayerController :type Player%20Controller%20Object%20Reference))
  (bind _returnvalue (Pawn|GetControlledPawn PlayerController))
  (Utilities|IsValid _returnvalue
    (:Is%20Valid
      (Actor|DestroyActor _returnvalue))
    (:Is%20Not%20Valid
      _))
  (bind _returnvalue_2 (Game|SpawnActorfromClass "/Game/ThirdPerson/Blueprints/BP_ThirdPersonCharacter.BP_ThirdPersonCharacter_C" (Spawning|FindPlayerStartTransform) "Undefined" "MultiplyWithRoot" 0 0))
  ;[1 1 1] Server call twice. May be a problem later
  (Variables|Default|SetPlayerstart_num (+ (Variables|Default|GetPlayerstart_num) 1))
  (Pawn|Possess PlayerController _returnvalue_2))

(fn GMUpdateScore
  (params (PlayerName :type String) (PlayerController :type Player%20Controller%20Object%20Reference))
  (for _array_element (Utilities|Array|MakeArray PlayerController)
    (CallFunction|SetScores PlayerName)))

(fn SetScores
  (params (Scorername :type String))
  (for _array_element (Variables|Default|GetAll_PartyGamePlayerControllers)
    (bind _aspartygame_multiplayer_playercontroller_bp (Utilities|Casting|CastToPartygame_multiplayer_playercontroller_BP _array_element)
      (:then
        (Variables|Default|SetAs%20Partygame%20Multiplayer%20Playercontroller%20BP _aspartygame_multiplayer_playercontroller_bp)
        (switch string Scorername
          (:Default
            (Development|PrintString (Utilities|String|Append Scorername "< failed scorer name") true true "(R=1.000000,G=0.000000,B=0.175211,A=1.000000)" 15.0))
          (:p1
            (Variables|/Game/Blueprints/GameMode/Partygame_multiplayer_playercontroller_BP.Partygame_multiplayer_playercontroller_BP_C|Setp1currentScore _aspartygame_multiplayer_playercontroller_bp (+ (Variables|/Game/Blueprints/GameMode/Partygame_multiplayer_playercontroller_BP.Partygame_multiplayer_playercontroller_BP_C|Getp1currentScore _aspartygame_multiplayer_playercontroller_bp) 1)))
          (:p2
            (Development|PrintString Scorername true true "(R=0.864183,G=0.990043,B=1.000000,A=1.000000)" 55.0)
            (Variables|/Game/Blueprints/GameMode/Partygame_multiplayer_playercontroller_BP.Partygame_multiplayer_playercontroller_BP_C|Setp2currentScore _aspartygame_multiplayer_playercontroller_bp (+ (Variables|/Game/Blueprints/GameMode/Partygame_multiplayer_playercontroller_BP.Partygame_multiplayer_playercontroller_BP_C|Getp2currentScore _aspartygame_multiplayer_playercontroller_bp) 1)))
          (:p3
            (Variables|/Game/Blueprints/GameMode/Partygame_multiplayer_playercontroller_BP.Partygame_multiplayer_playercontroller_BP_C|Setp3currentScore (Variables|Default|GetAs%20Partygame%20Multiplayer%20Playercontroller%20BP) (+ (Variables|/Game/Blueprints/GameMode/Partygame_multiplayer_playercontroller_BP.Partygame_multiplayer_playercontroller_BP_C|Getp3currentScore (Variables|Default|GetAs%20Partygame%20Multiplayer%20Playercontroller%20BP)) 1)))
          (:p4
            (Variables|/Game/Blueprints/GameMode/Partygame_multiplayer_playercontroller_BP.Partygame_multiplayer_playercontroller_BP_C|Setp4currentScore (Variables|Default|GetAs%20Partygame%20Multiplayer%20Playercontroller%20BP) (+ (Variables|/Game/Blueprints/GameMode/Partygame_multiplayer_playercontroller_BP.Partygame_multiplayer_playercontroller_BP_C|Getp4currentScore (Variables|Default|GetAs%20Partygame%20Multiplayer%20Playercontroller%20BP)) 1)))))
      (:CastFailed
        (Development|PrintString "Cast failed test scores")))))