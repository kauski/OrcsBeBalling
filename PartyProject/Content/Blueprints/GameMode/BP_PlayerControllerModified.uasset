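; Player controller for a multiplayer party game, handling each player's menus, input modes and session flow.
; On BeginPlay it applies saved screen settings from BP_SaveAudio and prepares the in-game menu, which Tab toggles during play.
; It relays ready and continue states to BP_GameModeModified and updates pre-game widgets.
; IsGameStarted switches between score UI and end screen; kicking destroys the session, and a debug key increments P1's GameState score.
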(event Custom|IncrementScore
  ;[1 1 1] Developer cheats
  (bind _asbp_game_state_modified (Utilities|Casting|CastToBP_GameStateModified (Game|GetGameState)))
  (Math|Integer|IncrementInt (Variables|/Game/Blueprints/GameMode/BP_GameStateModified.BP_GameStateModified_C|GetP1Score _asbp_game_state_modified)
    (:%20%20
      (Development|PrintString "P1 Score increased"))))

(event Custom|CheatScore
  ;[1 1 1] Developer cheats
  (bind _asbp_game_state_modified (Utilities|Casting|CastToBP_GameStateModified (Game|GetGameState)))
  (Math|Integer|IncrementInt (Variables|/Game/Blueprints/GameMode/BP_GameStateModified.BP_GameStateModified_C|GetP2Score _asbp_game_state_modified)
    (:%20%20
      (Development|PrintString "P2 Score increased"))))

(event Custom|IsGameStarted
  (params (GameStart :type Boolean))
  ;[1 1 1] Sets a boolean when game is started
  (Networking|SwitchHasAuthority
    (:Authority
      _)
    (:Remote
      _))
  (bind _output_get (Variables|Default|SetIsGameStartedd GameStart))
  (if _output_get
    (Utilities|IsValid (Variables|Default|GetGameUIRef)
      (:Is%20Valid
        (Development|PrintString "Game UI is valid")
        (Widget|SetVisibility (Variables|Default|GetGameUIRef) "Visible"))
      (:Is%20Not%20Valid
        (Development|PrintString "Game UI is not valid")
        (bind _returnvalue (UserInterface|CreateWidget "/Game/Blueprints/GameMode/Partygame_UI_WidgetModified.Partygame_UI_WidgetModified_C"))
        (UserInterface|Viewport|AddtoViewport _returnvalue 0)
        (bind _asgameplay_hud (Utilities|Casting|CastToGameplayHUD (HUD|GetHUD)))
        (Default|ScoreUIWidgetSetter _asgameplay_hud _returnvalue)
        (Variables|Default|SetGameUIRef _returnvalue)))
    (else
      (Widget|SetVisibility (Variables|Default|GetGameUIRef) "Collapsed")
      (CallFunction|DestroyMenu)
      (CallFunction|InitialControls)
      (bind _returnvalue_2 (UserInterface|CreateWidget "/Game/Blueprints/UI/W_EndScreen.W_EndScreen_C"))
      (UserInterface|Viewport|AddtoViewport _returnvalue_2 0))))

(event Custom|InitialControls
  ;[1 1 1] Initial controls function
  (Input|SetInputModeUIOnly (Game|GetPlayerController 0) 0 "DoNotLock" false))

(event Custom|OC_KickPlayer
  ;[1 1 1] Kick player function
  (Game|OpenLevel(byName) "L_InitialMap")
  (|DestroySession (Game|GetPlayerController 0)))

(event Custom|CreateWaitingWidget
  ;[1 1 1] Creates waiting screen widget
  (bind _returnvalue (UserInterface|CreateWidget "/Game/Blueprints/UI/W_WaitingScreen.W_WaitingScreen_C" (Game|GetPlayerController 0)))
  (UserInterface|Viewport|AddtoViewport _returnvalue 0))

(event Custom|ServerUpdatePlayersContinue
  (params (IsContinue :type Boolean))
  (bind _asbp_game_mode_modified (Utilities|Casting|CastToBP_GameModeModified (Game|GetGameMode)))
  (Default|SetPlayertoContinue _asbp_game_mode_modified self IsContinue)
  (Development|PrintString "Player is set to continue"))

(event Custom|SetPreGameMenuVisible
  ;[1 1 1] Sets the visibility of pregamemenu to visible
  (Widget|SetVisibility (Variables|Default|GetW_PreGameMenuRef) "Visible"))

(event Custom|PCUpdatePlayersContinue
  (params (IsContinue :type Array%20of%20Booleans))
  (bind _asbp_game_mode_modified (Utilities|Casting|CastToBP_GameModeModified (Game|GetGameMode)))
  (Default|UpdatePlayersContinue _asbp_game_mode_modified IsContinue))

(event Custom|SetScreenMode
  (params (WindowMod :type EWindowMode%20Enum :default "Fullscreen"))
  (bind _returnvalue (Settings|GetGameUserSettings))
  (Class|GameUserSettings|SetFullscreenMode _returnvalue WindowMod)
  (Class|GameUserSettings|ApplyResolutionSettings _returnvalue false)
  (Development|PrintString (Utilities|String|Append "Window mode at start is: " (Utilities|String|EnumtoString WindowMod))))

(event Custom|SetResolution
  (params (Window%20Mod :type EWindowMode%20Enum :default "Fullscreen") (AxisX :type String) (AxisY :type String))
  (bind _returnvalue (Settings|GetGameUserSettings))
  (Class|GameUserSettings|SetScreenResolution _returnvalue (Utilities|Struct|MakeIntPoint (Math|Conversions|ToInteger(Byte) AxisX) (Math|Conversions|ToInteger(Byte) AxisY)))
  (Class|GameUserSettings|SetFullscreenMode _returnvalue Window%20Mod)
  (Class|GameUserSettings|ApplyResolutionSettings _returnvalue false))

(event Custom|ExecuteOnce
  (bind _slot_name (Variables|Default|GetSlot%20Name))
  ;[1 1 1] Executes screen settings check once
  (if (not (Variables|Default|GetOnceBool))
    (bind _returnvalue (SaveGame|DoesSaveGameExist _slot_name))
    (if _returnvalue
      (bind _returnvalue_2 (SaveGame|LoadGamefromSlot _slot_name))
      (bind _asbp_save_audio (Utilities|Casting|CastToBP_SaveAudio _returnvalue_2))
      (bind _output_get (Variables|Default|SetSaveAudioRef _asbp_save_audio))
      (Variables|Default|SetbShowMouseCursor true)
      (CallFunction|SetScreenMode (Variables|/Game/Sounds/BP_SaveAudio.BP_SaveAudio_C|GetWindowMode _asbp_save_audio))
      (CallFunction|SetResolution (Variables|/Game/Sounds/BP_SaveAudio.BP_SaveAudio_C|GetWindowMode _asbp_save_audio) (Variables|/Game/Sounds/BP_SaveAudio.BP_SaveAudio_C|GetResolutionX _output_get) (Variables|/Game/Sounds/BP_SaveAudio.BP_SaveAudio_C|GetResolutionY _output_get))
      (Variables|Default|SetOnceBool true)
      (else
        (bind _returnvalue_3 (SaveGame|CreateSaveGameObject "/Game/Sounds/BP_SaveAudio.BP_SaveAudio_C"))
        (Variables|Default|SetSaveAudioRef _returnvalue_3)))))

(event Custom|GameControls
  ;[1 1 1] Game controls function
  (Input|SetInputModeGameandUI (Game|GetPlayerController 0) 0 "DoNotLock" false true))

(event Custom|UpdatePlayerList
  (params (PlayerInfoStruct :type Array%20of%20BP%20Player%20Info%20Struct%20Structures))
  ;[1 1 1] Updates player info struct
  (Variables|Default|SetAllPlayerInfo PlayerInfoStruct)
  (Networking|SwitchHasAuthority
    (:Authority
      _)
    (:Remote
      _))
  (bind _asw_pre_game_menu (Utilities|Casting|CastToW_PreGameMenu (Variables|Default|GetUserWidgetRef)))
  (Default|UpdateWidget _asw_pre_game_menu (Variables|Default|GetAllPlayerInfo)))

(event Custom|PauseControls
  ;[1 1 1] In game menu controls
  (Input|SetInputModeGameandUI (Game|GetPlayerController 0) 0 "DoNotLock" false false))

(event Custom|SetUserWidgetRef
  (params (Ref :type User%20Widget%20Object%20Reference) (Ref2 :type W%20Pre%20Game%20Menu%20Object%20Reference))
  ;[1 1 1] Sets user widget reference for casting to work
  (Variables|Default|SetUserWidgetRef Ref)
  (Variables|Default|SetW_PreGameMenuRef Ref2))

(event Custom|ServerUpdatePlayerReady
  (params (IsReady :type Boolean))
  ;[1 1 1] Updates ready players on server
  (bind _asbp_game_mode_modified (Utilities|Casting|CastToBP_GameModeModified (Game|GetGameMode)))
  (Default|SetPlayerReady _asbp_game_mode_modified self IsReady))

(event Custom|UpdatePlayerReady
  (params (IsReady :type Array%20of%20Booleans))
  (bind _w_pregamemenuref (Variables|Default|GetW_PreGameMenuRef))
  ;[1 1 1] Updates ready players for clients
  (Utilities|IsValid _w_pregamemenuref
    (:Is%20Valid
      (Default|UpdatePlayersReady _w_pregamemenuref IsReady))
    (:Is%20Not%20Valid
      (Development|PrintString "BP_PLAYERCONTROLLERMODIFIED NOT VALID"))))

(event Custom|MakeMenu
  ;[1 1 1] Show and hide the in game menu
  (Utilities|IsValid (Variables|Default|GetMenuRef)
    (:Is%20Valid
      (UserInterface|Viewport|AddtoViewport (Variables|Default|GetMenuRef) 0)
      (Widget|SetVisibility (Variables|Default|GetMenuRef) "Visible")
      (Variables|Default|SetIsPressed true))
    (:Is%20Not%20Valid
      (bind _returnvalue (UserInterface|CreateWidget "/Game/Blueprints/W_GameMenu.W_GameMenu_C"))
      (Variables|Default|SetMenuRef _returnvalue))))

(event Custom|DestroyMenu
  ;[1 1 1] Show and hide the in game menu
  (Widget|SetVisibility (stale Custom|MakeMenu _returnvalue) "Collapsed")
  (Variables|Default|SetIsPressed false))

(event EventBeginPlay
  ;[1 1 1] Beginplay
  (CallFunction|ExecuteOnce)
  (CallFunction|MakeMenu)
  (Variables|Default|Setp1currentScore 0)
  (Variables|Default|Setp2currentScore 0)
  (Variables|Default|Setp3currentScore 0)
  (Variables|Default|Setp4currentScore 0)
  (Variables|Default|SetcurrentScorer (Class|AdvancedSessionsLibrary|GetPlayerName self))
  (Utilities|Array|Add (Variables|Default|GetPlayerColors) "(R=1.000000,G=0.000000,B=0.000000,A=1.000000)")
  (Utilities|Array|Add (Variables|Default|GetPlayerColors) "(R=0.000000,G=1.000000,B=0.000000,A=1.000000)")
  (Utilities|Array|Add (Variables|Default|GetPlayerColors) "(R=0.000000,G=0.000000,B=1.000000,A=1.000000)")
  (Utilities|Array|Add (Variables|Default|GetPlayerColors) "(R=1.000000,G=0.000000,B=1.000000,A=1.000000)"))

(event Input|KeyboardEvents|DebugKeyG
  (params (Key :type Key%20Structure :default "None") (ActionValue :type Input%20Action%20Value%20Structure))
  ;[1 1 1] Developer cheats
  (:Pressed
    (CallFunction|IncrementScore)))

(event Input|KeyboardEvents|Tab
  (params (Key :type Key%20Structure :default "None"))
  ;[1 1 1] In game menu function
  (:Pressed
    (if (Variables|Default|GetIsGameStartedd)
      (if (Variables|Default|GetIsPressed)
        (Development|PrintString "GAME")
        (CallFunction|GameControls)
        (CallFunction|DestroyMenu)
        (else
          (Development|PrintString "MENU")
          (CallFunction|PauseControls)
          (CallFunction|MakeMenu)))
      (else
        (Development|PrintString "Game is not started yet!")))))

(fn ConstructionScript)

(fn OnRepP1currentScore)