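; Player controller for the multiplayer party game that requests player spawning and carries prototype score-reporting logic.
; On local BeginPlay it asks the game mode to spawn the player, sets Game-and-UI input, zeroes four scores and stores its player name as scorer.
; SR_ events forward score and scorer updates to game state or game mode, with some marked unused or left unwired.
; Debug keys trigger score updates and prints; OnRep handlers are empty.
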(event Custom|SR_SpawnPlayer
  ;[1 1 1] Server Player spawning
  (bind _aspartygame_multiplayer_gamemode_bp (Utilities|Casting|CastToPartygame_multiplayer_gamemode_BP (Game|GetGameMode)))
  (Default|SpawnPlayer _aspartygame_multiplayer_gamemode_bp self))

(event Custom|SR_CallUpdateScore
  (params (scorerName :type String))
  ;[1 1 1] ServerUpdateScore (Not used currently)
  (Networking|SwitchHasAuthority
    (:Authority
      (bind _aspartygame_multiplayer_gamestate_bp (Utilities|Casting|CastToPartygame_multiplayer_gamestateBP (Game|GetGameState)))
      (Default|SRUpdateScore _aspartygame_multiplayer_gamestate_bp)
      (Development|PrintString (Utilities|String|Append (Utilities|GetDisplayName (Game|GetPlayerController 0)) "< AAAAAAAAAAAAAAAAAAAAAA") true true "(R=1.000000,G=0.906680,B=0.000000,A=1.000000)" 15.0))))

(event Custom|SR_Scores
  (params (NewParam :type Integer))
  ;[1 1 1] ServerUpdateScore (Not used currently)
  (Variables|Default|Setp1currentScore NewParam))

(event Custom|SR_SetScorer
  (params (ScorerName :type String))
  ;[1 1 1] Setscorer (not used currently)
  (Development|PrintString "SR_SETSCORER CALLED")
  (bind _aspartygame_multiplayer_gamestate_bp (Utilities|Casting|CastToPartygame_multiplayer_gamestateBP (Game|GetGameState))
    (:then
      (Default|SRSetScorer _aspartygame_multiplayer_gamestate_bp ScorerName))
    (:CastFailed
      (Development|PrintString "Set scorer failed" true true "(R=1.000000,G=0.000000,B=0.332405,A=1.000000)" 44.0))))

(event Custom|SR_UpdateScore
  (params (Scorer%20name :type String))
  (bind _currentscorer (Variables|Default|GetcurrentScorer))
  ;[1 1 1] ServerUpdateScore (Not used currently)
  (Development|PrintString "UpdateScoreCalled" true true "(R=0.922404,G=1.000000,B=0.744632,A=1.000000)" 1e+01)
  (Development|PrintString (Utilities|String|Append "Current scorer: " _currentscorer) true true "(R=1.000000,G=1.000000,B=1.000000,A=1.000000)" 666.0)
  (bind _aspartygame_multiplayer_gamemode_bp (Utilities|Casting|CastToPartygame_multiplayer_gamemode_BP (Game|GetGameMode))
    (:then
      (Default|GMUpdateScore _aspartygame_multiplayer_gamemode_bp _currentscorer self))
    (:CastFailed
      (Development|PrintString "Cast failed"))))

(event EventBeginPlay
  ;[1 1 1] Beginplay Setters
  (if (Pawn|IsLocalController)
    (CallFunction|SRSpawnPlayer)
    (Variables|Default|SetbShowMouseCursor true)
    (Input|SetInputModeGameandUI self 0 "LockAlways" false false)
    (Variables|Default|Setp1currentScore 0)
    (Variables|Default|Setp2currentScore 0)
    (Variables|Default|Setp3currentScore 0)
    (Variables|Default|Setp4currentScore 0)
    (Variables|Default|SetcurrentScorer (Class|AdvancedSessionsLibrary|GetPlayerName self))))

(event Input|KeyboardEvents|1
  (params (Key :type Key%20Structure :default "None"))
  ;[1 1 1] Debug bindingei
  (:Pressed
    (CallFunction|SRCallUpdateScore (Variables|Default|GetcurrentScorer))))

(event Input|KeyboardEvents|F
  (params (Key :type Key%20Structure :default "None"))
  (:Pressed
    ;[1 1 1] Debug bindingei
    (Development|PrintString (Class|AdvancedSessionsLibrary|GetPlayerName self) true true "(R=0.291187,G=0.000000,B=1.000000,A=1.000000)" 4.0)))

(event Input|KeyboardEvents|2
  (params (Key :type Key%20Structure :default "None"))
  ;[1 1 1] Debug bindingei
  (:Pressed
    (CallFunction|SRCallUpdateScore (Variables|Default|GetcurrentScorer))))

(event Input|KeyboardEvents|3
  (params (Key :type Key%20Structure :default "None"))
  ;[1 1 1] Debug bindingei
  (:Pressed
    (CallFunction|SRCallUpdateScore (Variables|Default|GetcurrentScorer))))

(event Input|KeyboardEvents|J
  (params (Key :type Key%20Structure :default "None"))
  ;[1 1 1] Debug bindingei
  (:Pressed
    (bind _aspartygame_multiplayer_gamestate_bp (Utilities|Casting|CastToPartygame_multiplayer_gamestateBP (Game|GetGameState)))
    (Default|PrintScorer _aspartygame_multiplayer_gamestate_bp)))

(event Input|KeyboardEvents|C
  (params (Key :type Key%20Structure :default "None"))
  (:Pressed
    ;[1 1 1] Debug bindingei
    (bind _aspartygame_multiplayer_gamestate_bp (Utilities|Casting|CastToPartygame_multiplayer_gamestateBP (Game|GetGameState)))
    (Default|PrintArray _aspartygame_multiplayer_gamestate_bp)))

(fn ConstructionScript)

(fn GetActorSoundParams
  (return 0))

(fn OnRepP2currentScore)

(fn ReturnIngamename
  (return (Variables|Default|GetIngamename)))

(fn OnRepP1currentScore)

(fn OnRepCurrentScorer)