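; Game state for a multiplayer ball-throwing game with a pre-game lobby and scoring for up to four players.
; Events switch the local player controller between lobby and game controls, collapsing the pre-game menu on start.
; A replicated player list's OnRep refreshes lobby widgets from the controller's player info.
; SR_ events record scorer and thrower, increment the current scorer's tally, and forward ball pickups and throws to the character.
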(event Custom|SR_UpdateScore
  ;[1 1 1] Update score
  (if true
    (Development|PrintString "ADDING SCORE")
    (switch string (Variables|Default|GetcurrentScorer)
      (:Default
        (Development|PrintString "Something went wrong in gamestate switch" true true "(R=1.000000,G=0.000000,B=0.182047,A=1.000000)" 15.0))
      (:p1
        (Variables|Default|SetP1Score (+ (Variables|Default|GetP1Score) 1)))
      (:p2
        (Variables|Default|SetP2Score (+ (Variables|Default|GetP2Score) 1)))
      (:p3
        (Variables|Default|SetP3Score (+ (Variables|Default|GetP3Score) 1)))
      (:p4
        (Variables|Default|SetP4Score (+ (Variables|Default|GetP4Score) 1))))))

(event Custom|SR_SetScorer
  (params (scorer :type String))
  ;[1 1 1] Setscorer
  (bind _output_get (Variables|Default|SetcurrentScorer scorer))
  (Development|PrintString (Utilities|String|Append "In gamestate scorer set to: " _output_get) true true "(R=0.000000,G=1.000000,B=0.125474,A=1.000000)" 55.0))

(event Custom|UpdatePlayerList
  ;[1 1 1] Updates player list array
  (Variables|Default|SetAllPlayerStates (Variables|Default|GetPlayerArray)))

(event Custom|PlusOne
  (params (number :type Integer))
  ;[1 1 1] plus one
  (Math|Integer|IncrementInt number))

(event Custom|RestartGame
  ;[1 1 1] Restarts the game into the lobby state again
  (Networking|SwitchHasAuthority
    (:Authority
      _)
    (:Remote
      _))
  (bind _asbp_player_controller_modified (Utilities|Casting|CastToBP_PlayerControllerModified (Game|GetPlayerController 0)))
  (Default|InitialControls _asbp_player_controller_modified)
  (Default|IsGameStarted _asbp_player_controller_modified false))

(event Custom|SR_SetThrower
  (params (throwerName :type String))
  ;[1 1 1] SetThrower
  (bind _output_get (Variables|Default|SetcurrentThrower throwerName))
  (Development|PrintString (Utilities|String|Append "In gamestate thrower set to: " _output_get) true true "(R=0.000000,G=1.000000,B=0.125474,A=1.000000)" 55.0))

(event Custom|SR_PlayerThrew
  (params (playerController :type BP%20Player%20Controller%20Modified%20Object%20Reference))
  (bind _asbp_third_person_character (Utilities|Casting|CastToBP_ThirdPersonCharacter (Pawn|GetControlledPawn playerController))
    (:then
      (Default|SetHasBall _asbp_third_person_character playerController))
    (:CastFailed
      (Development|PrintString "lmao"))))

(event Custom|SR_PickedUpBall
  (params (playerController :type BP%20Player%20Controller%20Modified%20Object%20Reference))
  (bind _asbp_third_person_character (Utilities|Casting|CastToBP_ThirdPersonCharacter (Pawn|GetControlledPawn playerController))
    (:then
      (Default|SetHasBall _asbp_third_person_character playerController))
    (:CastFailed
      (Development|PrintString "MC failed" true true "(R=1.000000,G=0.000000,B=0.148993,A=1.000000)" 2222.0))))

(event Custom|UpdatePlayerUI
  ;[1 1 1] removes the lobby UI when host starts game
  (bind _foundwidgets (Widget|GetAllWidgetsOfClass "/Game/Blueprints/UI/W_PreGameMenu.W_PreGameMenu_C" false))
  (for _array_element _foundwidgets
    (Widget|SetVisibility _array_element "Collapsed")
    (bind _asbp_player_controller_modified (Utilities|Casting|CastToBP_PlayerControllerModified (Game|GetPlayerController 0)))
    (Default|GameControls _asbp_player_controller_modified)
    (Default|IsGameStarted _asbp_player_controller_modified true)))

(event EventBeginPlay
  ;[1 1 1] adds the initial UI only controls
  (bind _asbp_player_controller_modified (Utilities|Casting|CastToBP_PlayerControllerModified (Game|GetPlayerController 0)))
  (Default|InitialControls _asbp_player_controller_modified))

(fn ConstructionScript)

(fn OnRepAllPlayerStates
  (bind _foundwidgets (Widget|GetAllWidgetsOfClass "/Game/Blueprints/UI/W_PreGameMenu.W_PreGameMenu_C" false))
  (bind _asbp_player_controller_modified (Utilities|Casting|CastToBP_PlayerControllerModified (Game|GetPlayerController 0)))
  (for _array_element _foundwidgets
    (Default|UpdateWidget _array_element (Variables|/Game/Blueprints/GameMode/BP_PlayerControllerModified.BP_PlayerControllerModified_C|GetAllPlayerInfo _asbp_player_controller_modified))))