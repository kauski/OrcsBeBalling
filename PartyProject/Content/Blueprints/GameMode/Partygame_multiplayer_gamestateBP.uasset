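; Game state for a multiplayer party game, holding the current thrower, current scorer and scores for four players.
; SR_ events set thrower and scorer, and SR_UpdateScore switches on the scorer's name to increment that player's score, with heavy debug printing.
; These values have RepNotify functions, but only the scorer's does anything: it clears CurrentScorer on player controller 0.
; BeginPlay also caches all PlayerStart actors.
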(event Custom|SR_UpdateScore
  ;[1 1 1] Update score
  (if true
    (Development|PrintString "ADDING SCORE")
    (switch string (Variables|Default|GetcurrentScorer)
      (:Default
        (Development|PrintString "Something went wrong in gamestate switch" true true "(R=1.000000,G=0.000000,B=0.182047,A=1.000000)" 15.0))
      (:p1
        (Variables|Default|SetP1Score (+ (Variables|Default|GetP1Score) 1)))
      (:p2
        (Variables|Default|SetP2Score (+ (Variables|Default|GetP2Score) 1)))
      (:p3
        (Variables|Default|SetP3Score (+ (Variables|Default|GetP3Score) 1)))
      (:p4
        (Variables|Default|SetP4Score (+ (Variables|Default|GetP4Score) 1))))))

(event Custom|SR_SetScorer
  (params (scorer :type String))
  ;[1 1 1] Setscorer
  (bind _output_get (Variables|Default|SetcurrentScorer scorer))
  (Development|PrintString (Utilities|String|Append "In gamestate scorer set to: " _output_get) true true "(R=0.000000,G=1.000000,B=0.125474,A=1.000000)" 55.0))

(event Custom|PrintScorer
  ;[1 1 1] Debug printing
  (Development|PrintString (Variables|Default|GetcurrentScorer) true true "(R=0.000000,G=1.000000,B=0.357936,A=1.000000)" 15.0))

(event Custom|PlusOne
  (params (number :type Integer))
  (Math|Integer|IncrementInt number))

(event Custom|Print%20array
  ;[1 1 1] Debug printing
  (Development|PrintString (Utilities|String|Append (Utilities|String|ToString(Boolean) (Utilities|Enum|Equal(Enum) (Variables|Default|GetcurrentScorer) (Variables|Default|GetcurrentThrower))) "<<<<< booli")))

(event Custom|SR_SetThrower
  (params (throwerName :type String))
  ;[1 1 1] SetThrower
  (bind _output_get (Variables|Default|SetcurrentThrower throwerName))
  (Development|PrintString (Utilities|String|Append "In gamestate thrower set to: " _output_get) true true "(R=0.000000,G=1.000000,B=0.125474,A=1.000000)" 55.0))

(event EventBeginPlay
  ;[1 1 1] Beginplay
  (bind _outactors (Actor|GetAllActorsOfClass "/Script/Engine.PlayerStart"))
  (Variables|Default|SetOut%20Actors _outactors))

(event EventTick
  (params (DeltaSeconds :type Float%20%28single-precision%29)))

(fn ConstructionScript)

(fn OnRepP4Score)

(fn OnRepP1Score)

(fn OnRepP2Score)

(fn OnRepP3Score)

(fn OnRepCurrentScorer
  (bind _aspartygame_multiplayer_playercontroller_bp (Utilities|Casting|CastToPartygame_multiplayer_playercontroller_BP (Game|GetPlayerController 0)))
  (Variables|/Game/Blueprints/GameMode/Partygame_multiplayer_playercontroller_BP.Partygame_multiplayer_playercontroller_BP_C|SetcurrentScorer _aspartygame_multiplayer_playercontroller_bp ""))

(fn OnRepCurrentThrower)