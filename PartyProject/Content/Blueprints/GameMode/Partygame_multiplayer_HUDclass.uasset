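; HUD class for the multiplayer party game that shows player scores in a Partygame_UI_Widget.
; BeginPlay creates the widget for the owning player and adds it to the viewport.
; SR_UpdateScore switches on player name to write name and score, though all four cases target P1ScoreText.
; UpdateMyScore prints the given name and calls SetScores on the game mode with an empty string.
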(event Custom|SR_UpdateScore
  (params (Player :type String) (CurrentScore :type Integer))
  (switch string Player
    (:Default
      (Development|PrintString "Switch broke" true true "(R=0.000000,G=1.000000,B=0.175124,A=1.000000)" 3e+01))
    (:p1
      (for _array_element (Variables|Default|GetAllScoreWidgets)
        (Rendering|Components|TextRender|SetText (Variables|/Game/Blueprints/GameMode/Partygame_UI_Widget.Partygame_UI_Widget_C|GetP1_Score_text (Variables|Default|GetScore_UI_Widget)) (Utilities|Text|ToText(String) (Utilities|String|Append Player (Utilities|String|ToString(Integer) CurrentScore))))))
    (:p2
      (Rendering|Components|TextRender|SetText (Variables|/Game/Blueprints/GameMode/Partygame_UI_Widget.Partygame_UI_Widget_C|GetP1_Score_text (Variables|Default|GetScore_UI_Widget)) (Utilities|Text|ToText(String) (Utilities|String|Append Player (Utilities|String|ToString(Integer) CurrentScore)))))
    (:p3
      (Rendering|Components|TextRender|SetText (Variables|/Game/Blueprints/GameMode/Partygame_UI_Widget.Partygame_UI_Widget_C|GetP1_Score_text (Variables|Default|GetScore_UI_Widget)) (Utilities|Text|ToText(String) (Utilities|String|Append Player (Utilities|String|ToString(Integer) CurrentScore)))))
    (:p4
      (Rendering|Components|TextRender|SetText (Variables|/Game/Blueprints/GameMode/Partygame_UI_Widget.Partygame_UI_Widget_C|GetP1_Score_text (Variables|Default|GetScore_UI_Widget)) (Utilities|Text|ToText(String) (Utilities|String|Append Player (Utilities|String|ToString(Integer) CurrentScore)))))))

(event Custom|UpdateMyScore
  (params (Name :type String))
  (Development|PrintString Name)
  (bind _aspartygame_multiplayer_gamemode_bp (Utilities|Casting|CastToPartygame_multiplayer_gamemode_BP (Game|GetGameMode)))
  (Default|SetScores _aspartygame_multiplayer_gamemode_bp))

(event Collision|EventActorBeginOverlap
  (params (OtherActor :type Actor%20Object%20Reference)))

(event EventTick
  (params (DeltaSeconds :type Float%20%28single-precision%29)))

(event EventBeginPlay
  (bind _returnvalue (UserInterface|CreateWidget "/Game/Blueprints/GameMode/Partygame_UI_Widget.Partygame_UI_Widget_C" (Game|Player|GetOwningPlayerController)))
  (bind _output_get (Variables|Default|SetScore_UI_Widget _returnvalue))
  (UserInterface|Viewport|AddtoViewport _output_get 0)
  (Widget|GetAllWidgetsOfClass "/Game/Blueprints/GameMode/Partygame_UI_Widget.Partygame_UI_Widget_C" true))

(fn ConstructionScript)