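; GI_GamePlay, apparently the game instance, hosts multiplayer sessions and switches input modes for pausing and starting play.
; HostServer creates an Advanced Session with a random eight-digit ServerName and an IsPrivate flag set through SetPrivateLobby, then opens the level as a listen server.
; Pausing only sets UI-only input on player 0.
; Starting calls StartGameInputMode on that controller, then repeats it through MultiSetGameStarted.
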(event Custom|SetGameStarted
  ;[1 1 1] Start game function to set input mode game only
  (bind _asoldbp_player_controller_modified (Utilities|Casting|CastToOLDBP_PlayerControllerModified (Game|GetPlayerController 0))
    (:then
      (Default|StartGameInputMode _asoldbp_player_controller_modified)
      (CallFunction|MultiSetGameStarted))
    (:CastFailed
      (Development|PrintString "Start Game Input Mode CAST FAILED!"))))

(event Custom|SetGamePaused
  ;[1 1 1] Pause game function to set input mode UI only
  (Input|SetInputModeUIOnly (Game|GetPlayerController 0) 0 "DoNotLock" false))

(event Custom|SetPrivateLobby
  ;[1 1 1] Setting private lobby
  (Variables|Default|SetIsPrivateGI true))

(event Custom|Host%20Server
  (params (PlayerController :type Player%20Controller%20Object%20Reference) (PublicConnections :type Integer) (bUseLAN :type Boolean) (LevelName :type Name))
  ;[1 1 1] make a server with random code consisting of 8 numbers
  (|AdvancedSession (Utilities|Array|MakeArray (Class|AdvancedSessionsLibrary|MakeLiteralSessionPropertyString "ServerName" (Utilities|String|ToString(Integer) (Math|Random|RandomIntegerinRange 10000000 99999999))) (Class|AdvancedSessionsLibrary|MakeLiteralSessionPropertyBool "IsPrivate" (Variables|Default|GetIsPrivateGI))) PlayerController PublicConnections 0 bUseLAN true false true true true false false false true false true
    (:OnSuccess
      (Utilities|String|LogString "Created a Session from GI_GamePlay")
      (Game|OpenLevel(byName) LevelName true "listen"))))

(event Custom|MultiSetGameStarted
  (bind _asoldbp_player_controller_modified (Utilities|Casting|CastToOLDBP_PlayerControllerModified (Game|GetPlayerController 0))
    (:then
      (Default|StartGameInputMode _asoldbp_player_controller_modified))
    (:CastFailed
      (Development|PrintString "Start Game Input Mode CAST FAILED!"))))