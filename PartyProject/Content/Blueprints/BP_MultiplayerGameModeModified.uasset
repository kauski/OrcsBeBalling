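; Multiplayer game mode that tracks connected player controllers and manages their player list, pawns and kicking.
; Login and logout edit the controller array, then trigger a briefly delayed player-list update on the game state.
; Spawn routines create and possess third-person characters at a fixed location for controllers lacking pawns, and kicking uses the array index.
; Other events refresh all controllers or collapse a passed widget through server- and multicast-named handlers.
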(event Custom|UpdatePlayerList
  ;[1 1 1] updates playerlist to gamestate
  (Utilities|FlowControl|Delay 0.3)
  (bind _asbp_game_state_modified (Utilities|Casting|CastToOLDBP_GameStateModified (Game|GetGameState)))
  (Default|UpdatePlayerList _asbp_game_state_modified))

(event Custom|SetHiddenWidgetServer
  (params (UserWidgetRef :type User%20Widget%20Object%20Reference))
  (Widget|SetVisibility UserWidgetRef "Collapsed")
  (Development|PrintString "Server set widget to collapsed")
  (CallFunction|SetHiddenWidgetMulticast UserWidgetRef))

(event Custom|SetHiddenWidgetMulticast
  (params (UserWidgetRef :type User%20Widget%20Object%20Reference))
  (Widget|SetVisibility UserWidgetRef "Collapsed")
  (Development|PrintString "Client set widget to collapsed"))

(event Custom|UpdatePlayerControllers
  (Utilities|FlowControl|Delay 0.3)
  (for _array_element (Variables|Default|GetAll_PlayerControllers)
    (bind _asbp_player_controller_modified (Utilities|Casting|CastToOLDBP_PlayerControllerModified _array_element))
    (Default|UpdatePlayerControllers _asbp_player_controller_modified)))

(event EventPostLogin
  (params (NewPlayer :type Player%20Controller%20Object%20Reference))
  ;[1 1 1] adds to the array of connected players and removes logged out players from the array
  (bind _asbp_player_controller_modified (Utilities|Casting|CastToOLDBP_PlayerControllerModified NewPlayer))
  (Utilities|Array|Add (Variables|Default|GetAll_PlayerControllers) _asbp_player_controller_modified)
  (CallFunction|UpdatePlayerList))

(event EventOnLogout
  (params (ExitingController :type Controller%20Object%20Reference))
  ;[1 1 1] adds to the array of connected players and removes logged out players from the array
  (bind _asbp_player_controller_modified (Utilities|Casting|CastToOLDBP_PlayerControllerModified ExitingController))
  (Utilities|Array|RemoveItem (Variables|Default|GetAll_PlayerControllers) _asbp_player_controller_modified)
  (CallFunction|UpdatePlayerList))

(event EventHandleStartingNewPlayer
  (params (NewPlayer :type Player%20Controller%20Object%20Reference))
  ;[1 1 1] Create characters for controllers
  (for _array_element (Variables|Default|GetAll_PlayerControllers)
    (Utilities|IsValid (Pawn|GetControlledPawn _array_element)
      (:Is%20Not%20Valid
        (bind _returnvalue (Game|SpawnActorfromClass "/Game/ThirdPerson/Blueprints/BP_ThirdPersonCharacter.BP_ThirdPersonCharacter_C" (Math|Transform|MakeTransform "0.000000,0.000000,202.000000" "0, 0, 0" "1.000000,1.000000,1.000000") "Undefined" "MultiplyWithRoot" 0 0))
        (Pawn|Possess _array_element _returnvalue)))))

(fn ConstructionScript)

(fn KickPlayer
  (params (PlayerID :type Integer))
  ;[1 1 1] kick correct player with player ID
  (Default|OCKickPlayer (Utilities|Array|Get(acopy) (Variables|Default|GetAll_PlayerControllers) PlayerID)))

(fn SpawnCharacters
  (params (PlayerControllerRef :type Player%20Controller%20Object%20Reference))
  (for _array_element (Variables|Default|GetAll_PlayerControllers)
    (Utilities|IsValid (Pawn|GetControlledPawn _array_element)
      (:Is%20Valid
        (return))
      (:Is%20Not%20Valid
        (bind _returnvalue (Game|SpawnActorfromClass "/Game/ThirdPerson/Blueprints/BP_ThirdPersonCharacter.BP_ThirdPersonCharacter_C" (Math|Transform|MakeTransform "0.000000,0.000000,202.000000" "0, 0, 0" "1.000000,1.000000,1.000000") "Undefined" "MultiplyWithRoot" 0 0))
        (Pawn|Possess _array_element _returnvalue)))))