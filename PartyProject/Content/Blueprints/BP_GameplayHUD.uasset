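; Gameplay HUD Blueprint that opens the pre-game menu on BeginPlay and handles player score display.
; It stores a score widget passed in through a setter, which SR_UpdateScore fills with player name plus score.
; All four player cases write to P1ScoreText; P 1 loops AllScoreWidgets but still updates only the stored widget.
; UpdateMyScore prints the given name and calls SetScore on BP_GameModeModified with an empty string.
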(event Custom|SR_UpdateScore
  (params (Player :type String) (CurrentScore :type Integer))
  (switch string Player
    (:Default
      (Development|PrintString "Switch broke" true true "(R=0.000000,G=1.000000,B=0.175124,A=1.000000)" 3e+01))
    (:p1
      (for _array_element (Variables|Default|GetAllScoreWidgets)
        (Rendering|Components|TextRender|SetText (Variables|/Game/Blueprints/GameMode/Partygame_UI_WidgetModified.Partygame_UI_WidgetModified_C|GetP1_Score_text (Variables|Default|GetScore_UI_Widget)) (Utilities|Text|ToText(String) (Utilities|String|Append Player (Utilities|String|ToString(Integer) CurrentScore))))))
    (:p2
      (Rendering|Components|TextRender|SetText (Variables|/Game/Blueprints/GameMode/Partygame_UI_WidgetModified.Partygame_UI_WidgetModified_C|GetP1_Score_text (Variables|Default|GetScore_UI_Widget)) (Utilities|Text|ToText(String) (Utilities|String|Append Player (Utilities|String|ToString(Integer) CurrentScore)))))
    (:p3
      (Rendering|Components|TextRender|SetText (Variables|/Game/Blueprints/GameMode/Partygame_UI_WidgetModified.Partygame_UI_WidgetModified_C|GetP1_Score_text (Variables|Default|GetScore_UI_Widget)) (Utilities|Text|ToText(String) (Utilities|String|Append Player (Utilities|String|ToString(Integer) CurrentScore)))))
    (:p4
      (Rendering|Components|TextRender|SetText (Variables|/Game/Blueprints/GameMode/Partygame_UI_WidgetModified.Partygame_UI_WidgetModified_C|GetP1_Score_text (Variables|Default|GetScore_UI_Widget)) (Utilities|Text|ToText(String) (Utilities|String|Append Player (Utilities|String|ToString(Integer) CurrentScore)))))))

(event Custom|UpdateMyScore
  (params (Name :type String))
  (Development|PrintString Name)
  (bind _asbp_game_mode_modified (Utilities|Casting|CastToBP_GameModeModified (Game|GetGameMode)))
  (Default|SetScore _asbp_game_mode_modified))

(event Custom|ScoreUIWidgetSetter
  (params (ScoreUIWidget :type Partygame%20UI%20Widget%20Modified%20Object%20Reference))
  (Variables|Default|SetScore_UI_Widget ScoreUIWidget))

(event EventBeginPlay
  (bind _returnvalue (UserInterface|CreateWidget "/Game/Blueprints/UI/W_PreGameMenu.W_PreGameMenu_C" (Game|GetPlayerController 0)))
  (UserInterface|Viewport|AddtoViewport _returnvalue 0))

(fn ConstructionScript)